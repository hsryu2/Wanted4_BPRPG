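; BP_Bear is a monster Blueprint that takes damage, flashes when struck and dissolves on death.
; Incoming damage goes to BPHpController, whose dead event switches the state, disables capsule collision and plays a death timeline before destroying the actor.
; Timelines drive the mesh material's HitValue and Dissolve parameters, with the hit flash triggered by overlapping actors tagged PlayerWeapon, separately from damage handling.
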(event Custom|ReceiveOnDead
  (bind _mesh (Variables|Character|GetMesh))
  ;[0.15 0.02711 0 0.5] 죽음 이벤트에 바인딩
  (Variables|Default|SetState_BP "NewEnumerator3")
  (Collision|SetCollisionEnabled (Variables|Collision|GetCapsuleComponent) "NoCollision")
  (bind (_direction _dissolve _hitvalue) (Timeline|DeathEffect PlayFromStart)
    (:Update
      (Rendering|Material|SetScalarParameterValueonMaterials _mesh "Dissolve" _dissolve)
      (Rendering|Material|SetScalarParameterValueonMaterials _mesh "HitValue" _hitvalue))
    (:Finished
      (Actor|DestroyActor))))

(event EventBeginPlay
  ;[0.15 0.02711 0 0.5] 죽음 이벤트에 바인딩
  (EventDispatchers|BindEventtoOnDeadEvent (Variables|Default|GetBP_HpController) (delegate Custom|ReceiveOnDead)))

(event Collision|EventActorBeginOverlap
  (params (OtherActor :type Actor%20Object%20Reference))
  (if (Actor|ActorHasTag OtherActor "PlayerWeapon")
    (bind _hitvalue (Timeline|HitEffect PlayFromStart)
      (:Update
        (Rendering|Material|SetScalarParameterValueonMaterials (Variables|Character|GetMesh) "HitValue" _hitvalue)))))

(event EventTick
  (params (DeltaSeconds :type Float%20%28single-precision%29)))

(event Game|Damage|EventAnyDamage
  (params (Damage :type Float%20%28single-precision%29) (DamageType :type Damage%20Type%20Object%20Reference) (InstigatedBy :type Controller%20Object%20Reference) (DamageCauser :type Actor%20Object%20Reference))
  (Default|ReceiveDamage (Variables|Default|GetBP_HpController) Damage))

(fn ConstructionScript)